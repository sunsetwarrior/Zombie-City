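; Zombie enemy for ZombieCity that roams the navmesh, chases pawns it sees and damages the player.
; PawnSensing starts an AI move toward the seen pawn and removes one player HP as that move begins, not on arrival.
; Tick starts random roam moves while out of range, gated by a Running flag, and shows zombie HP on a TextRender.
; A death event destroys the zombie when its HP is depleted.
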(event `self.PawnSensing.OnSeePawn`
  (params (Pawn :type "Pawn Object Reference"))
  (set `self.In Range` true)
  (bind _aspawn (cast `Pawn` Pawn))
  (`|AIMoveTo` self (0.0 0.0 0.0) _aspawn
    (:`then`
      (`self.Remove_Player_HP`))
    (:`OnSuccess`
      (set `self.In Range` false))))

(event `self.ReceiveTick`
  (params (DeltaSeconds :type "Float (single-precision)"))
  (bind _ai_003_hp (`self.AI_003_HP`))
  (`|ExecutionSequence`
    (:`then_0`
      (if (`self.In Range`)
        _
        (elif (not (`self.Running`))
          (`|AIMoveTo` self (`NavigationSystem.GetRandomPointInNavigableRadius` (`self.Origin`) 5000.0) (stale `self.PawnSensing.OnSeePawn` _aspawn)
            (:`then`
              (set `self.Running` true))
            (:`OnSuccess`
              (set `self.Running` false :!label _label))
            (:`OnFail`
              (goto _label))))))
    (:`then_1`
      (`KismetSystemLibrary.PrintString` (`KismetStringLibrary.Conv_IntToString` _ai_003_hp) false true (struct :`R` 0.104348 :`G` 1.0 :`B` 0.151156 :`A` 1.0))
      (`TextRenderComponent.K2_SetText` (`self.TextRender`) (`KismetTextLibrary.Conv_IntToText` _ai_003_hp)))))

(event `AI_003_die`
  (if (<= (`self.AI_003_HP`) 0)
    (`self.K2_DestroyActor`)))

(event `Remove_Player_HP`
  (bind _aszombie_city_pawn (cast `/Game/ZombieCity/Blueprints/ZombieCityPawn` (stale `self.PawnSensing.OnSeePawn` Pawn)))
  (set `/Game/ZombieCity/Blueprints/ZombieCityPawn.Player_HP` (- (`/Game/ZombieCity/Blueprints/ZombieCityPawn.Player_HP` _aszombie_city_pawn) 1) _aszombie_city_pawn)
  (`/Game/ZombieCity/Blueprints/ZombieCityPawn.Player_Die` _aszombie_city_pawn))

(fn `UserConstructionScript`)